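; Checkpoint actor that records a teleport location in the Soundless game instance when the third-person character enters its box.
; A one-time overlap saves the Cylinder's world location as TeleportSet and increments the TeleportPoint counter.
; It then teleports the checkpoint actor itself to that location and shows a second cylinder for a second as feedback.
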(event OnComponentBeginOverlap(Box)
  (params (OverlappedComponent :type Primitive%20Component%20Object%20Reference) (OtherActor :type Actor%20Object%20Reference) (OtherComp :type Primitive%20Component%20Object%20Reference) (OtherBodyIndex :type Integer) (bFromSweep :type Boolean) (SweepResult :type Hit%20Result%20Structure%20%28by%20ref%29))
  (bind _gmi_instance (Variables|Default|GetGMI_Instance))
  (Utilities|Casting|CastToThirdPersonCharacter OtherActor)
  (Utilities|FlowControl|DoOnce false
    (:Completed
      (Variables|/Game/Thibaud/Blueprints/GMI_Soundless.GMI_Soundless_C|SetTeleportSet _gmi_instance (Transformation|GetWorldLocation (Variables|Default|GetCylinder)))
      (Variables|/Game/Thibaud/Blueprints/GMI_Soundless.GMI_Soundless_C|SetTeleport_Point _gmi_instance (+ (Variables|/Game/Thibaud/Blueprints/GMI_Soundless.GMI_Soundless_C|GetTeleport_Point _gmi_instance) 1))
      (Transformation|Teleport (Variables|/Game/Thibaud/Blueprints/GMI_Soundless.GMI_Soundless_C|GetTeleportSet _gmi_instance) "0, 0, 0")
      (Rendering|SetVisibility (Variables|Default|GetCylinder1) true false)
      (Utilities|FlowControl|Delay 1.0)
      (Rendering|SetVisibility (Variables|Default|GetCylinder1) false false))))

(event EventBeginPlay
  (bind _asgmi_soundless (Utilities|Casting|CastToGMI_Soundless (Game|GetGameInstance)))
  (Variables|Default|SetGMI_Instance _asgmi_soundless))

(fn ConstructionScript)