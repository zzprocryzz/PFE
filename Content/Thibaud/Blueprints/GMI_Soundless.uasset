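; GMI_Soundless, apparently the game instance Blueprint for Soundless, holds music-related state flags and provides an event to reset them.
; The Reset_VariableMusique event uses a Sequence to set four groups of five booleans (X, Y, B and A) to false, one group per output.
; The file shows no logic that sets these flags to true or reads them.
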(event Custom|Reset_VariableMusique
  (Utilities|FlowControl|Sequence
    (:then_0
      (Variables|Button_Musics|SetX1 false)
      (Variables|Button_Musics|SetX2 false)
      (Variables|Button_Musics|SetX3 false)
      (Variables|Button_Musics|SetX4 false)
      (Variables|Button_Musics|SetX5 false))
    (:then_1
      (Variables|Button_Musics|SetY1 false)
      (Variables|Button_Musics|SetY2 false)
      (Variables|Button_Musics|SetY3 false)
      (Variables|Button_Musics|SetY4 false)
      (Variables|Button_Musics|SetY5 false))
    (:then_2
      (Variables|Button_Musics|SetB1 false)
      (Variables|Button_Musics|SetB2 false)
      (Variables|Button_Musics|SetB3 false)
      (Variables|Button_Musics|SetB4 false)
      (Variables|Button_Musics|SetB5 false))
    (:then_3
      (Variables|Button_Musics|SetA1 false)
      (Variables|Button_Musics|SetA2 false)
      (Variables|Button_Musics|SetA3 false)
      (Variables|Button_Musics|SetA4 false)
      (Variables|Button_Musics|SetA5 false))))