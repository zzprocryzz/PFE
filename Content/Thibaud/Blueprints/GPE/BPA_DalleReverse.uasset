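; GPE actor for a moving slab that shuttles its Cylinder component back and forth.
; The Move timeline starts on BeginPlay and drives the Cylinder's relative location without sweep.
; Each time the timeline finishes, the Reverse flag picks the next direction: after a short pause it either reverses or replays from the start, toggling the flag to keep the loop going.
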(event Custom|Reverse
  (bind _newtrack_0 (Timeline|Move Reverse)
    (:Update
      (Transformation|SetRelativeLocation (Variables|Default|GetCylinder) _newtrack_0 false false))
    (:Finished
      (if (Variables|Default|GetReverse?)
        (Utilities|FlowControl|Delay 2.0)
        (CallFunction|ReStart)
        (Variables|Default|SetReverse? false)
        (else
          (Utilities|FlowControl|Delay 2.0)
          (Variables|Default|SetReverse? true)
          (CallFunction|Reverse))))))

(event Custom|ReStart
  (bind _newtrack_0 (Timeline|Move PlayFromStart)
    (:Update
      (Transformation|SetRelativeLocation (Variables|Default|GetCylinder) _newtrack_0 false false))
    (:Finished
      (if (Variables|Default|GetReverse?)
        (Utilities|FlowControl|Delay 2.0)
        (CallFunction|ReStart)
        (Variables|Default|SetReverse? false)
        (else
          (Utilities|FlowControl|Delay 2.0)
          (Variables|Default|SetReverse? true)
          (CallFunction|Reverse))))))

(event EventBeginPlay
  (bind _newtrack_0 (Timeline|Move Play)
    (:Update
      (Transformation|SetRelativeLocation (Variables|Default|GetCylinder) _newtrack_0 false false))
    (:Finished
      (if (Variables|Default|GetReverse?)
        (Utilities|FlowControl|Delay 2.0)
        (CallFunction|ReStart)
        (Variables|Default|SetReverse? false)
        (else
          (Utilities|FlowControl|Delay 2.0)
          (Variables|Default|SetReverse? true)
          (CallFunction|Reverse))))))

(fn ConstructionScript)