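; BPA_Flower is a gameplay element actor whose flower can be raised once the MonterFleur event is called.
; A timeline moves the Fleur component's relative location, flags the flower as used and hides the Sphere indicator.
; Until then, Sphere1 overlaps show the indicator when the ThirdPersonCharacter enters and hide it when the character leaves.
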(event OnComponentBeginOverlap(Sphere1)
  (params (OverlappedComponent :type Primitive%20Component%20Object%20Reference) (OtherActor :type Actor%20Object%20Reference) (OtherComp :type Primitive%20Component%20Object%20Reference) (OtherBodyIndex :type Integer) (bFromSweep :type Boolean) (SweepResult :type Hit%20Result%20Structure%20%28by%20ref%29))
  (Utilities|Casting|CastToThirdPersonCharacter OtherActor)
  (if (not (Variables|Default|GetCheckUse?))
    (Rendering|SetVisibility (Variables|Default|GetSphere) true false)))

(event OnComponentEndOverlap(Sphere1)
  (params (OverlappedComponent :type Primitive%20Component%20Object%20Reference) (OtherActor :type Actor%20Object%20Reference) (OtherComp :type Primitive%20Component%20Object%20Reference) (OtherBodyIndex :type Integer))
  (Utilities|Casting|CastToThirdPersonCharacter OtherActor)
  (if (not (Variables|Default|GetCheckUse?))
    (Rendering|SetVisibility (Variables|Default|GetSphere) false false)))

(event Custom|MonterFleur
  (bind _upflower (Timeline|Animation Play)
    (:Update
      (Transformation|SetRelativeLocation (Variables|Default|GetFleur) _upflower false false)
      (Variables|Default|SetCheckUse? true)
      (Rendering|SetVisibility (Variables|Default|GetSphere) false false))))

(event EventBeginPlay)

(fn ConstructionScript)