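; BPA_MusicConnect is a gameplay element that acts as a one-time music connection point with a proximity indicator.
; Overlapping its Box shows the Sphere and leaving hides it, as long as MusiqueUse is false.
; ConnectionAll sends VerificationGPEMessage to the referenced Actor, then sets MusiqueUse and hides the Sphere, so overlaps no longer toggle it.
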(event OnComponentBeginOverlap(Box)
  (params (OverlappedComponent :type Primitive%20Component%20Object%20Reference) (OtherActor :type Actor%20Object%20Reference) (OtherComp :type Primitive%20Component%20Object%20Reference) (OtherBodyIndex :type Integer) (bFromSweep :type Boolean) (SweepResult :type Hit%20Result%20Structure%20%28by%20ref%29))
  (if (not (Variables|Default|GetMusiqueUse))
    (Rendering|SetVisibility (Variables|Default|GetSphere) true false)))

(event OnComponentEndOverlap(Box)
  (params (OverlappedComponent :type Primitive%20Component%20Object%20Reference) (OtherActor :type Actor%20Object%20Reference) (OtherComp :type Primitive%20Component%20Object%20Reference) (OtherBodyIndex :type Integer))
  (if (not (Variables|Default|GetMusiqueUse))
    (Rendering|SetVisibility (Variables|Default|GetSphere) false false)))

(event Custom|ConnectionAll
  (Class|BPIConnection|VerificationGPE(Message) (Variables|Default|GetActor?))
  (Variables|Default|SetMusiqueUse true)
  (Rendering|SetVisibility (Variables|Default|GetSphere) false false))

(fn ConstructionScript)