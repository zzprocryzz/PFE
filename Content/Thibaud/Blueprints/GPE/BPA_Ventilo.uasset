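; Fan gameplay actor (Ventilo) that launches the player character when it enters the Cylinder1 volume.
; The overlap event casts to ThirdPersonCharacter and applies LaunchVelocity, overriding horizontal and vertical velocity.
; A self-calling Reset event blinks the cylinder on timed delays, but BeginPlay is empty and nothing here starts that loop.
; The blink changes only visibility, and the launch does not check it.
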(event OnComponentBeginOverlap(Cylinder1)
  (params (OverlappedComponent :type Primitive%20Component%20Object%20Reference) (OtherActor :type Actor%20Object%20Reference) (OtherComp :type Primitive%20Component%20Object%20Reference) (OtherBodyIndex :type Integer) (bFromSweep :type Boolean) (SweepResult :type Hit%20Result%20Structure%20%28by%20ref%29))
  (bind _asthird_person_character (Utilities|Casting|CastToThirdPersonCharacter OtherActor))
  (Character|LaunchCharacter _asthird_person_character (Variables|Default|GetLaunch%20Velocity) true true))

(event Custom|Reset
  (Utilities|FlowControl|Delay 2.0)
  (Rendering|SetVisibility (Variables|Default|GetCylinder1) false false)
  (Utilities|FlowControl|Delay 2.0)
  (Rendering|SetVisibility (Variables|Default|GetCylinder1) true false)
  (Utilities|FlowControl|Delay 2.0)
  (CallFunction|Reset))

(event EventBeginPlay)

(fn ConstructionScript)