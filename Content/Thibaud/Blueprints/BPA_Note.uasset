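; BPA_Note is a collectible note pickup that levitates until the player picks it up.
; A Levitation timeline starts on BeginPlay and drives the Sphere's relative location.
; When the timeline finishes, a Reverse flag switches between reverse playback and restart, looping the floating motion.
; Overlapping the Collsion component with a ThirdPersonCharacter plays a 2D sound and destroys the actor.
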(event OnComponentBeginOverlap(Collsion)
  (params (OverlappedComponent :type Primitive%20Component%20Object%20Reference) (OtherActor :type Actor%20Object%20Reference) (OtherComp :type Primitive%20Component%20Object%20Reference) (OtherBodyIndex :type Integer) (bFromSweep :type Boolean) (SweepResult :type Hit%20Result%20Structure%20%28by%20ref%29))
  (Utilities|Casting|CastToThirdPersonCharacter OtherActor)
  ;[1 1 1] Sound Add
  (Audio|PlaySound2D 0 1.0 1.0 0.0 0 0)
  (Actor|DestroyActor))

(event Custom|Reverse
  ;[1 0 0.2783] Animation Note Lévitation
  (bind _levitation (Timeline|Levitation Reverse)
    (:Update
      (Transformation|SetRelativeLocation (Variables|Default|GetSphere) _levitation false false))
    (:Finished
      (if (Variables|Default|GetReverse?)
        (CallFunction|ReStart)
        (Variables|Default|SetReverse? false)
        (else
          (Variables|Default|SetReverse? true)
          (CallFunction|Reverse))))))

(event Custom|ReStart
  ;[1 0 0.2783] Animation Note Lévitation
  (bind _levitation (Timeline|Levitation PlayFromStart)
    (:Update
      (Transformation|SetRelativeLocation (Variables|Default|GetSphere) _levitation false false))
    (:Finished
      (if (Variables|Default|GetReverse?)
        (CallFunction|ReStart)
        (Variables|Default|SetReverse? false)
        (else
          (Variables|Default|SetReverse? true)
          (CallFunction|Reverse))))))

(event EventBeginPlay
  ;[1 0 0.2783] Animation Note Lévitation
  (bind _levitation (Timeline|Levitation Play)
    (:Update
      (Transformation|SetRelativeLocation (Variables|Default|GetSphere) _levitation false false))
    (:Finished
      (if (Variables|Default|GetReverse?)
        (CallFunction|ReStart)
        (Variables|Default|SetReverse? false)
        (else
          (Variables|Default|SetReverse? true)
          (CallFunction|Reverse))))))

(fn ConstructionScript)