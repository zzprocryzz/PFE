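; Wall-mounted musical receptacle that the player fills with three plant notes to trigger a linked actor.
; Each interaction spends a note from GMI_Soundless, reveals the next sphere and decrements the character's note counter.
; The third note sends ConnectionInstrumentMessage to the referenced Actor.
; VerificationGPE shows a sprite and flags the player hit; UnCheck clears both once the character's GPEHIT is false.
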(event Custom|UnCheck
  (bind _asthird_person_character (Utilities|Casting|CastToThirdPersonCharacter (Game|GetPlayerCharacter 0)))
  (if (not (Variables|/Game/ThirdPersonBP/Blueprints/ThirdPersonCharacter.ThirdPersonCharacter_C|GetGPEHIT _asthird_person_character))
    (Rendering|SetVisibility (Variables|Default|GetPaperSprite) false false)
    (Variables|Default|SetHitbyPlayer false)))

(event EventInteraction?
  (bind _returnvalue (Game|GetPlayerCharacter 0))
  (bind _gmi_soundless (Variables|Default|GetGMI_Soundless))
  (if (>= (Variables|/Game/Thibaud/Blueprints/GMI_Soundless.GMI_Soundless_C|GetNbre_NotePlante (Variables|Default|GetGMI_Soundless)) 1)
    (Variables|/Game/Thibaud/Blueprints/GMI_Soundless.GMI_Soundless_C|SetNbre_NotePlante _gmi_soundless (- (Variables|/Game/Thibaud/Blueprints/GMI_Soundless.GMI_Soundless_C|GetNbre_NotePlante _gmi_soundless) 1))
    (Variables|Default|SetClef (+ (Variables|Default|GetClef) 1))
    (if (== (Variables|Default|GetClef) 1)
      (Rendering|SetVisibility (Variables|Default|GetSphere1) true false)
      (bind _asthird_person_character (Utilities|Casting|CastToThirdPersonCharacter _returnvalue))
      (Variables|/Game/ThirdPersonBP/Blueprints/ThirdPersonCharacter.ThirdPersonCharacter_C|SetAffNote _asthird_person_character (- (Variables|/Game/ThirdPersonBP/Blueprints/ThirdPersonCharacter.ThirdPersonCharacter_C|GetAffNote _asthird_person_character) 1))
      (elif (== (Variables|Default|GetClef) 2)
        (Rendering|SetVisibility (Variables|Default|GetSphere2) true false)
        (bind _asthird_person_character_2 (Utilities|Casting|CastToThirdPersonCharacter _returnvalue))
        (Variables|/Game/ThirdPersonBP/Blueprints/ThirdPersonCharacter.ThirdPersonCharacter_C|SetAffNote _asthird_person_character_2 (- (Variables|/Game/ThirdPersonBP/Blueprints/ThirdPersonCharacter.ThirdPersonCharacter_C|GetAffNote _asthird_person_character_2) 1))
        (elif (== (Variables|Default|GetClef) 3)
          (Rendering|SetVisibility (Variables|Default|GetSphere3) true false)
          (bind _asthird_person_character_3 (Utilities|Casting|CastToThirdPersonCharacter _returnvalue))
          (Variables|/Game/ThirdPersonBP/Blueprints/ThirdPersonCharacter.ThirdPersonCharacter_C|SetAffNote _asthird_person_character_3 (- (Variables|/Game/ThirdPersonBP/Blueprints/ThirdPersonCharacter.ThirdPersonCharacter_C|GetAffNote _asthird_person_character_3) 1))
          (Class|BPIConnection|ConnectionInstrument(Message) (Variables|Default|GetActor?)))))))

(event EventVerificationGPE
  (Rendering|SetVisibility (Variables|Default|GetPaperSprite) true false)
  (Variables|Default|SetHitbyPlayer true))

(event EventBeginPlay
  (bind _asgmi_soundless (Utilities|Casting|CastToGMI_Soundless (Game|GetGameInstance)))
  (Variables|Default|SetGMI_Soundless _asgmi_soundless))

(fn ConstructionScript)