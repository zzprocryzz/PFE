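; BPA_Platforme is a moving platform actor whose Cube travels back and forth along a Spline.
; BeginPlay sets the Move timeline's play rate from Rate and starts it.
; Each timeline update maps Move to a distance along the spline, setting the Cube's local location and rotation.
; On finish, the Repeat flag alternates between reversing the timeline and replaying it from the start, producing an endless loop.
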(event Custom|RepeatSystem
  (bind _spline (Variables|Default|GetSpline))
  (bind _move (Timeline|Move Reverse)
    (:Update
      (Transformation|SetRelativeLocationAndRotation (Variables|Default|GetCube) (Spline|GetLocationatDistanceAlongSpline _spline (* _move (Spline|GetSplineLength _spline)) "Local") (Spline|GetRotationatDistanceAlongSpline _spline (* _move (Spline|GetSplineLength _spline)) "Local") false false))
    (:Finished
      (if (Variables|Default|GetRepeat)
        (Variables|Default|SetRepeat false)
        (CallFunction|Restart)
        (else
          (Variables|Default|SetRepeat true)
          (CallFunction|RepeatSystem))))))

(event Custom|Restart
  (bind _spline (Variables|Default|GetSpline))
  (bind _move (Timeline|Move PlayFromStart)
    (:Update
      (Transformation|SetRelativeLocationAndRotation (Variables|Default|GetCube) (Spline|GetLocationatDistanceAlongSpline _spline (* _move (Spline|GetSplineLength _spline)) "Local") (Spline|GetRotationatDistanceAlongSpline _spline (* _move (Spline|GetSplineLength _spline)) "Local") false false))
    (:Finished
      (if (Variables|Default|GetRepeat)
        (Variables|Default|SetRepeat false)
        (CallFunction|Restart)
        (else
          (Variables|Default|SetRepeat true)
          (CallFunction|RepeatSystem))))))

(event EventBeginPlay
  (bind _spline (Variables|Default|GetSpline))
  (Components|Timeline|SetPlayRate (Variables|Default|GetMove) (Variables|Default|GetRate))
  (bind _move (Timeline|Move Play)
    (:Update
      (Transformation|SetRelativeLocationAndRotation (Variables|Default|GetCube) (Spline|GetLocationatDistanceAlongSpline _spline (* _move (Spline|GetSplineLength _spline)) "Local") (Spline|GetRotationatDistanceAlongSpline _spline (* _move (Spline|GetSplineLength _spline)) "Local") false false))
    (:Finished
      (if (Variables|Default|GetRepeat)
        (Variables|Default|SetRepeat false)
        (CallFunction|Restart)
        (else
          (Variables|Default|SetRepeat true)
          (CallFunction|RepeatSystem))))))

(fn ConstructionScript)