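; BPA_NotePlante is a collectible plant note that hovers in the world until the player picks it up.
; A Levitation timeline moves the Sphere's relative location, alternating forward and reverse through a Reverse flag to loop the bobbing.
; Overlap by ThirdPersonCharacter increments the note count in GMI_Soundless, plays a sound, notifies the WG_CarnetSounds widget created at BeginPlay, then destroys the actor.
; The construction script shows or hides an arrow sprite based on ShowArrow.
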(event OnComponentBeginOverlap(Collsion)
  (params (OverlappedComponent :type Primitive%20Component%20Object%20Reference) (OtherActor :type Actor%20Object%20Reference) (OtherComp :type Primitive%20Component%20Object%20Reference) (OtherBodyIndex :type Integer) (bFromSweep :type Boolean) (SweepResult :type Hit%20Result%20Structure%20%28by%20ref%29))
  (bind _gmi_soudless (Variables|Default|GetGMI_Soudless))
  (Utilities|Casting|CastToThirdPersonCharacter OtherActor)
  (Variables|/Game/Thibaud/Blueprints/GMI_Soundless.GMI_Soundless_C|Setnbre_NotePlante _gmi_soudless (+ (Variables|/Game/Thibaud/Blueprints/GMI_Soundless.GMI_Soundless_C|Getnbre_NotePlante _gmi_soudless) 1))
  (Audio|PlaySound2D (Variables|Default|GetSounds?) 1.0 1.0 0.0 0 0)
  (Default|AffichageNotePlante (Variables|Default|GetWG_CarnetSound))
  (Actor|DestroyActor))

(event Custom|Reverse
  ;[1 0 0.2783] Animation Note Lévitation
  (bind _levitation (Timeline|Levitation Reverse)
    (:Update
      (Transformation|SetRelativeLocation (Variables|Default|GetSphere) _levitation false false))
    (:Finished
      (if (Variables|Default|GetReverse?)
        (CallFunction|ReStart)
        (Variables|Default|SetReverse? false)
        (else
          (Variables|Default|SetReverse? true)
          (CallFunction|Reverse))))))

(event Custom|ReStart
  ;[1 0 0.2783] Animation Note Lévitation
  (bind _levitation (Timeline|Levitation PlayFromStart)
    (:Update
      (Transformation|SetRelativeLocation (Variables|Default|GetSphere) _levitation false false))
    (:Finished
      (if (Variables|Default|GetReverse?)
        (CallFunction|ReStart)
        (Variables|Default|SetReverse? false)
        (else
          (Variables|Default|SetReverse? true)
          (CallFunction|Reverse))))))

(event EventBeginPlay
  (bind _asgmi_soundless (Utilities|Casting|CastToGMI_Soundless (Game|GetGameInstance)))
  (Variables|Default|SetGMI_Soudless _asgmi_soundless)
  (bind _returnvalue (UserInterface|CreateWidget "/Game/Thibaud/Blueprints/Widgets/WG_CarnetSounds.WG_CarnetSounds_C"))
  ;[1 0 0.2783] Animation Note Lévitation
  (Variables|Default|SetWG_CarnetSound _returnvalue)
  (bind _levitation (Timeline|Levitation Play)
    (:Update
      (Transformation|SetRelativeLocation (Variables|Default|GetSphere) _levitation false false))
    (:Finished
      (if (Variables|Default|GetReverse?)
        (CallFunction|ReStart)
        (Variables|Default|SetReverse? false)
        (else
          (Variables|Default|SetReverse? true)
          (CallFunction|Reverse))))))

(fn ConstructionScript
  (if (Variables|Default|GetShow%20Arrow?)
    (Rendering|SetVisibility (Variables|Default|GetPaperSprite) true false)
    (else
      (Rendering|SetVisibility (Variables|Default|GetPaperSprite) false false))))