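; BPA_Nenuphar is a lily pad gameplay element that moves its Cylinder component along a timeline-driven path.
; VerificationGPE plays the Move timeline at a configurable rate, feeding its track into the cylinder's relative location.
; When Loop is set, each finish alternates between reversing and restarting after separate delays, using a Reverse flag to produce back-and-forth motion.
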(event Custom|Reverse
  (bind _newtrack_0 (Timeline|Move Reverse)
    (:Update
      (Transformation|SetRelativeLocation (Variables|Default|GetCylinder) _newtrack_0 false false))
    (:Finished
      (if (Variables|Default|Getloop?)
        (if (Variables|Default|GetReverse?)
          (Utilities|FlowControl|Delay (Variables|Default|GetTimer_Restart))
          (CallFunction|ReStart)
          (Variables|Default|SetReverse? false)
          (else
            (Utilities|FlowControl|Delay (Variables|Default|GetTimer_Reverse))
            (Variables|Default|SetReverse? true)
            (CallFunction|Reverse)))))))

(event Custom|ReStart
  (bind _newtrack_0 (Timeline|Move PlayFromStart)
    (:Update
      (Transformation|SetRelativeLocation (Variables|Default|GetCylinder) _newtrack_0 false false))
    (:Finished
      (if (Variables|Default|Getloop?)
        (if (Variables|Default|GetReverse?)
          (Utilities|FlowControl|Delay (Variables|Default|GetTimer_Restart))
          (CallFunction|ReStart)
          (Variables|Default|SetReverse? false)
          (else
            (Utilities|FlowControl|Delay (Variables|Default|GetTimer_Reverse))
            (Variables|Default|SetReverse? true)
            (CallFunction|Reverse)))))))

(event EventBeginPlay)

(event EventVerificationGPE
  (Components|Timeline|SetPlayRate (Variables|Default|GetMove) (Variables|Default|GetNewRate))
  (bind _newtrack_0 (Timeline|Move Play)
    (:Update
      (Transformation|SetRelativeLocation (Variables|Default|GetCylinder) _newtrack_0 false false))
    (:Finished
      (if (Variables|Default|Getloop?)
        (if (Variables|Default|GetReverse?)
          (Utilities|FlowControl|Delay (Variables|Default|GetTimer_Restart))
          (CallFunction|ReStart)
          (Variables|Default|SetReverse? false)
          (else
            (Utilities|FlowControl|Delay (Variables|Default|GetTimer_Reverse))
            (Variables|Default|SetReverse? true)
            (CallFunction|Reverse)))))))

(fn ConstructionScript)